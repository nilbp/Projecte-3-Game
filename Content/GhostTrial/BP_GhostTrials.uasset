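; BP_GhostTrials is a self-destroying ghost afterimage of the player character, frozen in the pose it has at spawn.
; On BeginPlay it replaces every material on the Fantasminha mesh with dynamic instances of MI_GhostTrial and copies the pose from the player's skeletal mesh.
; An Opacity timeline drives that parameter on all the instances and destroys the actor when it finishes.
; The pose copy and timeline restart sit inside the per-material loop.
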(event `self.ReceiveBeginPlay`
  (bind _asthird_person_character (cast `/Game/ThirdPersonBP/Blueprints/Character/CharacterMesh/ThirdPersonCharacter` (`GameplayStatics.GetPlayerPawn` 0)))
  (set `self.PlayerRef` _asthird_person_character)
  (`self.GhostTrial`))

(event `GhostTrial`
  (for _ (`MeshComponent.GetMaterials` (`self.Fantasminha`))
    (bind _returnvalue (`KismetMaterialLibrary.CreateDynamicMaterialInstance` "/Game/GhostTrial/MI_GhostTrial.MI_GhostTrial"))
    (bind _returnvalue_2 (`KismetArrayLibrary.Array_Add` (`self.DynamicMats`) _returnvalue))
    (`PrimitiveComponent.SetMaterial` (`self.Fantasminha`) _returnvalue_2 _returnvalue)
    (`PoseableMeshComponent.CopyPoseFromSkeletalComponent` (`self.Fantasminha`) (`Character.Mesh` (`self.PlayerRef`)))
    (bind (_direction _opacity) (`Timeline|Opacity` :!via `PlayFromStart`)
      (:`Update`
        (for _array_element (`self.DynamicMats`)
          (`MaterialInstanceDynamic.SetScalarParameterValue` _array_element "Opacity" _opacity)))
      (:`Finished`
        (`self.K2_DestroyActor` self)))))

(fn `UserConstructionScript`)